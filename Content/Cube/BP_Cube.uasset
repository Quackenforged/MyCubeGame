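; Player cube for an obstacle-dodging runner that is pushed forward along X and steered sideways by axis input.
; A looping timer applies forward velocity-change impulses while CanMove is set, and the same flag gates steering.
; Tick derives Score from X position, and BeginPlay adds the scoreboard widget.
; Hitting a BPObstacle sets CanMove to true, so movement is not halted, then reloads the current level after RestartDelay.
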(event OnComponentHit(Cube)
  (params (HitComponent :type Primitive%20Component%20Object%20Reference) (OtherActor :type Actor%20Object%20Reference) (OtherComp :type Primitive%20Component%20Object%20Reference) (NormalImpulse :type Vector :default "0, 0, 0") (Hit :type Hit%20Result%20Structure%20%28by%20ref%29))
  (Utilities|Casting|CastToBPObstacle OtherActor)
  (Variables|Default|SetCanMove? true)
  (Utilities|FlowControl|Delay (Variables|Default|GetRestartDelay))
  (bind _returnvalue (Game|GetCurrentLevelName true))
  (Game|OpenLevel(byName) (Utilities|String|StringToName _returnvalue)))

(event Custom|MoveCube
  (if (Variables|Default|GetCanMove?)
    (Physics|AddImpulse (Variables|Default|GetCube) (Math|Vector|MakeVector (Variables|Default|GetForwardForce) 0.0 0.0) "None" true)))

(event EventBeginPlay
  (bind _returnvalue (UserInterface|CreateWidget "/Game/Cube/BP_ScoreBoard.BP_ScoreBoard_C"))
  (UserInterface|Viewport|AddtoViewport _returnvalue 0)
  (Utilities|Time|SetTimerbyEvent (delegate Custom|MoveCube) 0.1 true))

(event EventTick
  (params (DeltaSeconds :type Float%20%28single-precision%29))
  (Variables|Default|SetScore (Math|Float|Truncate (/ (.x (Transformation|GetWorldLocation (Variables|Default|GetCube))) 1e+02))))

(event Input|AxisEvents|InputAxisMoveRight/Left
  (params (AxisValue :type Float%20%28single-precision%29))
  (if (Variables|Default|GetCanMove?)
    (Physics|AddImpulse (Variables|Default|GetCube) (Math|Vector|MakeVector 0.0 (* AxisValue (Variables|Default|GetMoveRight/LeftForce)) 0.0) "None" true)))

(fn ConstructionScript)